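; Bomb actor that starts a countdown when play begins and stands as an obstacle once the player moves off it.
; BeginPlay calls StartTime to set the trigger flag, and Tick then decrements Timer by delta time.
; At zero it only prints "Boom", repeating every frame because the flag is never cleared.
; When a TopDownCharacter ends overlap, the static mesh switches its Pawn channel response to Block.
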(event EventBeginPlay
  (CallFunction|StartTime))

(event Collision|EventActorBeginOverlap
  (params (OtherActor :type Actor%20Object%20Reference)))

(event EventTick
  (params (DeltaSeconds :type Float%20%28single-precision%29))
  (if (Variables|Default|GetIsTriggered)
    (bind _output_get (Variables|Default|SetTimer (- (Variables|Default|GetTimer) DeltaSeconds)))
    (if (<= _output_get 0.0)
      (Development|PrintString "Boom"))))

(event Collision|EventActorEndOverlap
  (params (OtherActor :type Actor%20Object%20Reference))
  ;[1 1 1] Attiva la collisione con il canale della fisica delle pawn appena il player smette di collidere
  (if (Utilities|ClassIsChildOf (Utilities|GetClass OtherActor) "/Game/TopDownBP/Blueprints/TopDownCharacter.TopDownCharacter_C")
    (Collision|SetCollisionResponsetoChannel (Variables|Debug|GetStaticMeshComponent) "ECC_Pawn" "ECR_Block")))

(fn ConstructionScript)

(fn StartTime
  (Variables|Default|SetIsTriggered true))