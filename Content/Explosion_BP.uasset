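; Explosion actor that travels in a straight line along its Direction variable, scaled by Velocity.
; Tick adds that step to the root's world location and writes it back as relative location, without sweep or delta-time scaling, so speed depends on frame rate.
; On overlap it filters out Bomb_BP actors and checks for StaticMeshActor, but neither branch performs any action.
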(event EventBeginPlay)

(event Collision|EventActorBeginOverlap
  (params (OtherActor :type Actor%20Object%20Reference))
  (bind _returnvalue (Utilities|GetClass OtherActor))
  (if (not (Utilities|ClassIsChildOf _returnvalue "/Game/Bomb_BP.Bomb_BP_C"))
    (if (Utilities|ClassIsChildOf _returnvalue "/Script/Engine.StaticMeshActor")
      _)))

(event EventTick
  (params (DeltaSeconds :type Float%20%28single-precision%29))
  (Transformation|SetRelativeLocation (Variables|Default|GetDefaultSceneRoot) (+ (Transformation|GetWorldLocation (Variables|Default|GetDefaultSceneRoot)) (* (Variables|Default|GetDirection) (Variables|Default|GetVelocity))) false false))

(fn ConstructionScript)